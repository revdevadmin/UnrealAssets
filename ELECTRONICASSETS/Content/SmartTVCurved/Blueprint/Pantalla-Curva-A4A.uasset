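; Curved smart TV actor that lets a nearby player toggle video playback with the left mouse button.
; A Box overlap enables input for player 0 and end overlap disables it, each toggling the Mouse component's visibility.
; Clicks flip IsPlaying: playing rewinds MediaMovie to the start and spawns MediaSound at the actor's location.
; Pausing affects only the movie, as the spawned sound is never stopped.
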(event OnComponentBeginOverlap(Box)
  (params (OtherActor :type Actor%20Object%20Reference) (OtherComp :type Primitive%20Component%20Object%20Reference) (OtherBodyIndex :type Integer) (bFromSweep :type Boolean) (SweepResult :type Hit%20Result%20Structure%20%28by%20ref%29))
  ;[1 1 1] Sistema que detecta la entrada del personaje
  (Input|EnableInput (Game|GetPlayerController 0))
  (Rendering|ToggleVisibility (Variables|Components|GetMouse) false))

(event OnComponentEndOverlap(Box)
  (params (OtherActor :type Actor%20Object%20Reference) (OtherComp :type Primitive%20Component%20Object%20Reference) (OtherBodyIndex :type Integer))
  ;[1 1 1] Sistema que detecta la entrada del personaje
  (Input|DisableInput (Game|GetPlayerController 0))
  (Rendering|ToggleVisibility (Variables|Components|GetMouse) false))

(event EventBeginPlay)

(event EventActorBeginOverlap
  (params (OtherActor :type Actor%20Object%20Reference)))

(event EventTick
  (params (DeltaSeconds :type Float%20%28single-precision%29)))

(event Input|MouseEvents|LeftMouseButton
  (bind _media_movie (Variables|Media|GetMedia_Movie))
  ;[1 1 1] Esto es el mecanismo de TV
  (:Pressed
    (if (Math|Boolean|Equal(Boolean) true (Variables|Media|GetisPlaying))
      (Variables|Media|SetisPlaying false)
      (Sequencer|Player|Pause (Variables|Media|GetMedia_Movie))
      (else
        (Variables|Media|SetisPlaying true)
        (Class|MediaPlayer|Rewind _media_movie)
        (Media|MediaPlayer|Play _media_movie :!class /Script/MediaAssets.MediaPlayer)
        (Audio|PlaySoundatLocation (Variables|Media|GetMedia_Sound) (Transformation|GetActorLocation))))))

(fn ConstructionScript)